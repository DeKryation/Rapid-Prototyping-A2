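; BP_Checkpoint is a one-shot checkpoint that activates when a BP_MainGame actor overlaps its CheckpointTrigger.
; Activation sets IsActivated, swaps the flag mesh to the M_Active material and sets HasActiveCheckpoint on the game instance.
; The node that would store the checkpoint's transform as LastCheckpointTransform is disconnected, so no respawn location is saved here.
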(event `self.ReceiveBeginPlay`)

(event `self.ReceiveActorBeginOverlap`
  (params (OtherActor :type "Actor Object Reference")))

(event `self.ReceiveTick`
  (params (DeltaSeconds :type "Float (single-precision)")))

(event `self.CheckpointTrigger.OnComponentBeginOverlap`
  (params (OtherActor :type "Actor Object Reference") (OtherComp :type "PrimitiveComponent Object Reference") (OtherBodyIndex :type Integer) (bFromSweep :type Boolean) (SweepResult :type "HitResult Structure (by ref)"))
  (if (not (`self.bIsActivated`))
    (cast `/Game/Blueprints/BP_MainGame` OtherActor)
    (set `self.bIsActivated` true)
    (`PrimitiveComponent.SetMaterial` (`self.FlagMesh`) 0 "/Game/Blueprints/CheckPoint/M_Active.M_Active")
    (bind _asbp_game_instance (cast `/Game/Blueprints/CheckPoint/BP+GameInstance` (`GameplayStatics.GetGameInstance`)))
    (set `/Game/Blueprints/CheckPoint/BP+GameInstance.bHasActiveCheckpoint` true _asbp_game_instance)))

(fn `UserConstructionScript`)